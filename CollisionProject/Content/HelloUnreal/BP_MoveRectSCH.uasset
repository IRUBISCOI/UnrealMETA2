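; BP_MoveRectSCH is an actor that moves its static mesh around a square loop in the X-Z plane.
; Every Tick, a switch on the Direction variable nudges the mesh's relative location a fixed step right, up, left or down.
; When the mesh passes that side's limit, Direction advances to the next side, forming a simple state machine.
; Movement is per frame without delta-time scaling or sweep, so speed depends on frame rate.
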(event `self.ReceiveTick`
  (params (DeltaSeconds :type "Float (single-precision)"))
  (bind _staticmesh (`self.StaticMesh`))
  (bind (_relativelocation_x _relativelocation_y _relativelocation_z) (`KismetMathLibrary.BreakVector` (`SceneComponent.RelativeLocation` (`self.StaticMesh`))))
  (bind _relativelocation_x_2 (`KismetMathLibrary.BreakVector` (`SceneComponent.RelativeLocation` (`self.StaticMesh`))))
  (bind (_relativelocation_x_3 _relativelocation_y_2 _relativelocation_z_2) (`KismetMathLibrary.BreakVector` (`SceneComponent.RelativeLocation` (`self.StaticMesh`))))
  (bind _relativelocation_x_4 (`KismetMathLibrary.BreakVector` (`SceneComponent.RelativeLocation` (`self.StaticMesh`))))
  ;[1 1 1] Move Rectengle
  (switch `/Game/HelloUnreal/EN_MoveType` (`self.Direction`)
    (:`NewEnumerator0`
      (`SceneComponent.K2_AddRelativeLocation` _staticmesh (10.0 0.0 0.0) false false)
      (if (>= _relativelocation_x_4 1000.0)
        (set `self.Direction` "NewEnumerator1")))
    (:`NewEnumerator1`
      (`SceneComponent.K2_AddRelativeLocation` _staticmesh (0.0 0.0 10.0) false false)
      (if (>= _relativelocation_z 1000.0)
        (set `self.Direction` "NewEnumerator2")))
    (:`NewEnumerator2`
      (`SceneComponent.K2_AddRelativeLocation` _staticmesh (-10.0 0.0 0.0) false false)
      (if (<= _relativelocation_x_2 0.0)
        (set `self.Direction` "NewEnumerator3")))
    (:`NewEnumerator3`
      (`SceneComponent.K2_AddRelativeLocation` _staticmesh (0.0 0.0 -10.0) false false)
      (if (<= _relativelocation_z_2 0.0)
        (set `self.Direction` "NewEnumerator0")))))

(fn `UserConstructionScript`)