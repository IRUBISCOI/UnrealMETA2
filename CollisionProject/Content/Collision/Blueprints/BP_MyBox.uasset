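; BP_MyBox is a collision trigger that starts and stops movers while something overlaps its Cube component.
; Begin overlap plays every MoveRect element, plus LeftRight and RotationBall from inside that same loop, and end overlap stops them all.
; Overlap and hit events print the component, other actor and other component names for debugging.
; BeginPlay and the construction script do no work.
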(event `self.ReceiveBeginPlay`
  (`|ExecutionSequence`))

(event `self.Cube.OnComponentBeginOverlap`
  (params (OverlappedComponent :type "PrimitiveComponent Object Reference") (OtherActor :type "Actor Object Reference") (OtherComp :type "PrimitiveComponent Object Reference") (OtherBodyIndex :type Integer) (bFromSweep :type Boolean) (SweepResult :type "HitResult Structure (by ref)"))
  (`KismetSystemLibrary.PrintString` (`KismetStringLibrary.Concat_StrStr` "Overlap : " (`KismetSystemLibrary.GetDisplayName` OverlappedComponent) "//Actor : " (`KismetSystemLibrary.GetDisplayName` OtherActor) "//Component : " (`KismetSystemLibrary.GetDisplayName` OtherComp)))
  (for _array_element (`self.MoveRect`)
    (`/Game/HelloUnreal/BP_MoveRect.Play` _array_element)
    (`/Game/HelloUnreal/BP_MoveLeftRightCSH.Play` (`self.LeftRight`))
    (`/Game/HelloUnreal/BP_LotationBall.Play` (`self.RotationBall`))))

(event `self.Cube.OnComponentEndOverlap`
  (params (OverlappedComponent :type "PrimitiveComponent Object Reference") (OtherActor :type "Actor Object Reference") (OtherComp :type "PrimitiveComponent Object Reference") (OtherBodyIndex :type Integer))
  (`KismetSystemLibrary.PrintString` (`KismetStringLibrary.Concat_StrStr` "Overlap : " (`KismetSystemLibrary.GetDisplayName` OverlappedComponent) "//Actor : " (`KismetSystemLibrary.GetDisplayName` OtherActor) "//Component : " (`KismetSystemLibrary.GetDisplayName` OtherComp)))
  (`/Game/HelloUnreal/BP_MoveLeftRightCSH.Stop` (`self.LeftRight`))
  (`/Game/HelloUnreal/BP_LotationBall.Stop` (`self.RotationBall`))
  (for _array_element (`self.MoveRect`)
    (`/Game/HelloUnreal/BP_MoveRect.Stop` _array_element)))

(event `self.Cube.OnComponentHit`
  (params (HitComponent :type "PrimitiveComponent Object Reference") (OtherActor :type "Actor Object Reference") (OtherComp :type "PrimitiveComponent Object Reference") (NormalImpulse :type "Vector Structure") (Hit :type "HitResult Structure (by ref)"))
  (`KismetSystemLibrary.PrintString` (`KismetStringLibrary.Concat_StrStr` "Hit : " (`KismetSystemLibrary.GetDisplayName` HitComponent) "//Actor : " (`KismetSystemLibrary.GetDisplayName` OtherActor) "//Component : " (`KismetSystemLibrary.GetDisplayName` OtherComp))))

(fn `UserConstructionScript`)